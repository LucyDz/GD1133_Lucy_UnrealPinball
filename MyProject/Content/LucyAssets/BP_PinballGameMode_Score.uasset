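; Pinball game mode that handles scoring and ball lives.
; AddScore adds the given points to the score held in BP_PinballGameState.
; OnBallLost decrements the remaining balls in that game state, then calls SpawnBall while any are left, otherwise it only prints "Game Over".
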(event EventBeginPlay
  (|CallParentFunction))

(event EventTick
  (params (DeltaSeconds :type Float%20%28single-precision%29))
  (|CallParentFunction DeltaSeconds) ; This node is disabled and will not be called.\nDrag off pins to build functionality.
)

(event EventAddScore
  (params (Points :type Float%20%28double-precision%29))
  ;[0.15 0.15 0.15 0.5] Add Points Gained
  (bind _asbp_pinball_game_state (Utilities|Casting|CastToBP_PinballGameState (Game|GetGameState)))
  (Default|SetScore _asbp_pinball_game_state (+ (Variables|/Game/LucyAssets/BP_PinballGameState.BP_PinballGameState_C|GetScore _asbp_pinball_game_state) Points))
  (Development|PrintString "Score Added" true true "(R=1.000000,G=0.000000,B=0.855909,A=1.000000)"))

(event EventOnBallLost
  ;[0.15 0.15 0.15 0.5] Check Ball Lives
  (bind _asbp_pinball_game_state (Utilities|Casting|CastToBP_PinballGameState (Game|GetGameState)))
  (bind _result (Math|Integer|DecrementInt (Variables|/Game/LucyAssets/BP_PinballGameState.BP_PinballGameState_C|GetBallsRemaining _asbp_pinball_game_state))
    (:%20%20
      (Default|SetBalls _asbp_pinball_game_state _result)
      (if (> _result 0)
        (CallFunction|SpawnBall)
        (else
          (Development|PrintString "Game Over" true true "(R=1.000000,G=0.000000,B=0.011142,A=1.000000)"))))))

(fn ConstructionScript
  (|CallParentFunction))