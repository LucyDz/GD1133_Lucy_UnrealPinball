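; BP_Flipper is a flipper actor that swings its FlipperPivot between resting and flipped rotations.
; On BeginPlay it derives the flipped rotation as a quarter turn whose sign depends on the Direction enum, so one Blueprint covers both swing directions.
; The activate and deactivate events play and reverse a timeline, which lerps the pivot's relative rotation between the two poses.
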(event Custom|OnActivate_Event
  ;[0.15 0.15 0.15 0.5] Flipper Move
  (bind _0_1 (Timeline|0-1 Play)
    (:Update
      (Transformation|SetRelativeRotation (Variables|Default|GetFlipperPivot) (Math|Rotator|Lerp(Rotator) (Variables|Default|GetFlipperResting) (Variables|Default|GetFlipperFlipped) _0_1) false false))))

(event Custom|OnDeactivate_Event
  ;[0.15 0.15 0.15 0.5] Flipper Move
  (bind _0_1 (Timeline|0-1 Reverse)
    (:Update
      (Transformation|SetRelativeRotation (Variables|Default|GetFlipperPivot) (Math|Rotator|Lerp(Rotator) (Variables|Default|GetFlipperResting) (Variables|Default|GetFlipperFlipped) _0_1) false false))))

(event EventBeginPlay
  ;[0.15 0.15 0.15 0.5] Setup
  (bind _output_get (Variables|Default|SetFlipperResting "0, 0, 0"))
  (Variables|Default|SetFlipperFlipped (Math|Rotator|CombineRotators _output_get (Math|Rotator|SelectRotator "0.000000,-90.000000,0.000000" "0.000000,90.000000,0.000000" (Utilities|Enum|Equal(Enum) (Variables|Default|GetDirection) "NewEnumerator0")))))

(event Collision|EventActorBeginOverlap
  (params (OtherActor :type Actor%20Object%20Reference)))

(event EventTick
  (params (DeltaSeconds :type Float%20%28single-precision%29)))

(fn ConstructionScript)