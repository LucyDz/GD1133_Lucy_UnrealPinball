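; Free-play game mode for a pinball game, where losing a ball simply spawns another with no limit shown.
; AddScore casts the game state to BP_PinballGameState and adds the gained points to its Score.
; BeginPlay runs the parent logic, and both it and AddScore print debug messages.
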(event EventBeginPlay
  (|CallParentFunction)
  (Development|PrintString "GameMode: Freeplay"))

(event EventTick
  (params (DeltaSeconds :type Float%20%28single-precision%29))
  (|CallParentFunction DeltaSeconds) ; This node is disabled and will not be called.\nDrag off pins to build functionality.
)

(event EventAddScore
  (params (Points :type Float%20%28double-precision%29))
  ;[0.15 0.15 0.15 0.5] Add Points Gained
  (bind _asbp_pinball_game_state (Utilities|Casting|CastToBP_PinballGameState (Game|GetGameState)))
  (Default|SetScore _asbp_pinball_game_state (+ (Variables|/Game/LucyAssets/BP_PinballGameState.BP_PinballGameState_C|GetScore _asbp_pinball_game_state) Points))
  (Development|PrintString "Score Added" true true "(R=1.000000,G=0.000000,B=0.855909,A=1.000000)"))

(event EventOnBallLost
  (CallFunction|SpawnBall))

(fn ConstructionScript
  (|CallParentFunction))