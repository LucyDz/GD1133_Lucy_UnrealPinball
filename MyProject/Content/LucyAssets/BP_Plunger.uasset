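; Pinball plunger actor that pulls back while held and triggers a launch impulse on the ball when released.
; The hold event runs a timeline that lerps the plunger mesh between start and end positions.
; Release stops the timeline, moves the mesh with MoveComponentTo, and calls the impulse event on the cached BP_Pinball.
; A box overlap caches that ball reference, which is never cleared.
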(event OnComponentBeginOverlap(Box)
  (params (OverlappedComponent :type Primitive%20Component%20Object%20Reference) (OtherActor :type Actor%20Object%20Reference) (OtherComp :type Primitive%20Component%20Object%20Reference) (OtherBodyIndex :type Integer) (bFromSweep :type Boolean) (SweepResult :type Hit%20Result%20Structure%20%28by%20ref%29))
  (bind _asbp_pinball (Utilities|Casting|CastToBP_Pinball OtherActor))
  (Variables|Default|SetAs%20BP%20Pinball _asbp_pinball))

(event Custom|PlungerHold_Event
  (bind _0_1 (Timeline|Timeline PlayFromStart)
    (:Update
      (Transformation|SetRelativeLocation (Variables|Default|GetSM_Plunger) (Math|Vector|Lerp(Vector) (Variables|Default|GetStartPos) (Variables|Default|GetEndPos) _0_1) false false))))

(event Custom|PlungerRelease_Event
  (Utilities|FlowControl|Sequence
    (:then_0
      (bind _0_1 (Timeline|Timeline Stop)
        (:Update
          (Transformation|SetRelativeLocation (Variables|Default|GetSM_Plunger) (Math|Vector|Lerp(Vector) (Variables|Default|GetStartPos) (Variables|Default|GetEndPos) _0_1) false false))))
    (:then_1
      (Components|MoveComponentTo (Variables|Default|GetSM_Plunger) "0, 0, 0" "0, 0, 0" false false 0.2 false)
      (Default|PinballImpulseEvent (Variables|Default|GetAs%20BP%20Pinball) "0, 0, 0"))))

(event EventBeginPlay)

(event Collision|EventActorBeginOverlap
  (params (OtherActor :type Actor%20Object%20Reference)))

(event EventTick
  (params (DeltaSeconds :type Float%20%28single-precision%29)))

(fn ConstructionScript)