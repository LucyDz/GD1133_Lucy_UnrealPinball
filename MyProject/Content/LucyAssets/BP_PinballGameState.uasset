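; Game state Blueprint for a pinball game that tracks the score and the number of balls remaining.
; BeginPlay resets the score to zero and sets the starting ball count through the SetScore and SetBalls events.
; Each setter stores the new value, broadcasts it through its OnScoreChanged or OnBallsChanged dispatcher, and prints it with PrintString.
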(event Custom|SetScore
  (params (NewScore :type Float%20%28double-precision%29))
  ;[0.15 0.15 0.15 0.5] Set New Score
  (bind _output_get (Variables|Default|SetScore NewScore))
  (Default|CallOnScoreChanged _output_get)
  (Development|PrintString (Utilities|String|ToString(Float) _output_get) true true "(R=0.252274,G=1.000000,B=0.000000,A=1.000000)"))

(event Custom|SetBalls
  (params (NewBalls :type Integer))
  ;[0.15 0.15 0.15 0.5] Set New Balls Remaining
  (bind _output_get (Variables|Default|SetBallsRemaining NewBalls))
  (Default|CallOnBallsChanged _output_get)
  (Development|PrintString (Utilities|String|ToString(Integer) _output_get) true true "(R=0.010330,G=0.467784,B=0.262251,A=1.000000)"))

(event EventBeginPlay
  (Utilities|FlowControl|Sequence
    (:then_0
      (CallFunction|SetScore 0.0))
    (:then_1
      (CallFunction|SetBalls 3))))

(event EventTick
  (params (DeltaSeconds :type Float%20%28single-precision%29)))

(fn ConstructionScript)