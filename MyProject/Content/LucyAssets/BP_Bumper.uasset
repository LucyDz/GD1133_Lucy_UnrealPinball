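; BP_Bumper is a pinball pop bumper that knocks reactive actors away and awards points.
; Capsule overlap sends an outward impulse through BPI_PinballReactive, then adds score via the game mode's BPI_ScoreReceiver.
; A timeline animates the bumper mechanism on any overlap, spawning a Niagara fire effect on every update.
; End overlap stops the timeline and snaps the mechanism back to its start position.
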(event OnComponentBeginOverlap(Capsule)
  (params (OverlappedComponent :type Primitive%20Component%20Object%20Reference) (OtherActor :type Actor%20Object%20Reference) (OtherComp :type Primitive%20Component%20Object%20Reference) (OtherBodyIndex :type Integer) (bFromSweep :type Boolean) (SweepResult :type Hit%20Result%20Structure%20%28by%20ref%29))
  (bind _returnvalue (Transformation|GetActorLocation))
  (Utilities|FlowControl|Sequence
    (:then_0
      ;[0.15 0.15 0.15 0.5] Apply Pinball Force
      (bind _asbpi_pinball_reactive (Utilities|Casting|CastToBPI_PinballReactive OtherActor))
      (Default|PinballImpulseEvent _asbpi_pinball_reactive (* (Variables|Default|GetMaxForce) (Math|Vector|Normalize (- (Transformation|GetWorldLocation OtherComp) _returnvalue))))
      ;[0.15 0.15 0.15 0.5] AddScore
      (bind _asbpi_score_receiver (Utilities|Casting|CastToBPI_ScoreReceiver (Game|GetGameMode)))
      (Default|AddScore _asbpi_score_receiver (Variables|Default|GetScoreValue)))
    (:then_1
      ;[0.15 0.15 0.15 0.5] Play Anim
      (bind _0_1 (Timeline|Timeline PlayFromStart)
        (:Update
          (Transformation|SetRelativeLocation (Variables|Default|GetSM_PopBumperMechanism) (Math|Vector|Lerp(Vector) (Variables|Default|GetStartPos) (Variables|Default|GetEndPos) _0_1) false false)
          (Niagara|SpawnSystematLocation "/Game/LucyAssets/Particles/NS_StylizedFireBumper.NS_StylizedFireBumper" _returnvalue "-11.000000,0.000000,0.000000"))))))

(event OnComponentEndOverlap(Capsule)
  (params (OverlappedComponent :type Primitive%20Component%20Object%20Reference) (OtherActor :type Actor%20Object%20Reference) (OtherComp :type Primitive%20Component%20Object%20Reference) (OtherBodyIndex :type Integer))
  (Utilities|FlowControl|Sequence
    (:then_0
      ;[0.15 0.15 0.15 0.5] Play Anim
      (bind _0_1 (Timeline|Timeline Stop)
        (:Update
          (Transformation|SetRelativeLocation (Variables|Default|GetSM_PopBumperMechanism) (Math|Vector|Lerp(Vector) (Variables|Default|GetStartPos) (Variables|Default|GetEndPos) _0_1) false false)
          (Niagara|SpawnSystematLocation "/Game/LucyAssets/Particles/NS_StylizedFireBumper.NS_StylizedFireBumper" (Transformation|GetActorLocation) "-11.000000,0.000000,0.000000"))))
    (:then_1
      (Transformation|SetRelativeLocation (Variables|Default|GetSM_PopBumperMechanism) (Variables|Default|GetStartPos) false false))))

(event EventBeginPlay)

(event Collision|EventActorBeginOverlap
  (params (OtherActor :type Actor%20Object%20Reference)))

(event EventTick
  (params (DeltaSeconds :type Float%20%28single-precision%29)))

(fn ConstructionScript)